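; Swinging door that can be opened normally or kicked open to either side, with 2D sounds for each action.
; Timelines rotate Scene1's yaw, with play rates set by open durations, and a kick starts from the last normal-open yaw.
; StopOpen halts opening and its sound, finished openings start a close timer, and Close swings the door back.
; GetIsFront uses a dot product to tell which side a location is on.
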(event `self.ReceiveBeginPlay`
  (`TimelineComponent.SetPlayRate` (`self.TL_KickOpen`) (/ 1.0 (`self.KickOpenSpeed`)))
  (`TimelineComponent.SetPlayRate` (`self.TL_NormalOpen`) (/ 1.0 (`self.normalOpenSpeed`))))

(event `NormalOpen`
  (params (isFront :type Boolean) (normalOpenSpeed :type "Float (double-precision)"))
  (set `self.isFront` isFront)
  (`|ExecutionSequence`
    (:`then_0`
      (set `self.normalOpenSpeed` normalOpenSpeed)
      (`TimelineComponent.SetPlayRate` (`self.TL_NormalOpen`) (/ 1.0 (`self.normalOpenSpeed`))))
    (:`then_1`
      (`|ExecutionSequence`
        (:`then_0`
          (bind (_direction _alpha) (`Timeline|TL_NormalOpen` :!via `PlayFromStart`)
            (:`Update`
              (set `self.currentYaw` (`KismetMathLibrary.Lerp` 0.0 (`KismetMathLibrary.SelectFloat` -90.0 90.0 (`self.isFront`)) _alpha))
              (`SceneComponent.K2_SetRelativeRotation` (`self.Scene1`) (`KismetMathLibrary.MakeRotator` 0.0 0.0 (`self.currentYaw`)) false false))
            (:`Finished`
              (`self.SetCloseTimer`))))
        (:`then_1`
          (bind _returnvalue (`GameplayStatics.SpawnSound2D` "/Game/Sound/DoorOpen.DoorOpen" 1.0 1.0 0.0 null))
          (set `self.openSound` _returnvalue))
        (:`then_2`
          (set `self.isOpen` true))))))

(event `KickOpen`
  (params (isFront :type Boolean) (KickOpenSpeed :type "Float (double-precision)"))
  (set `self.isFront` isFront)
  (`|ExecutionSequence`
    (:`then_0`
      (set `self.KickOpenSpeed` KickOpenSpeed)
      (`TimelineComponent.SetPlayRate` (`self.TL_KickOpen`) (/ 1.0 (`self.KickOpenSpeed`))))
    (:`then_1`
      (`|ExecutionSequence`
        (:`then_0`
          (bind (_direction _alpha) (`Timeline|TL_KickOpen` :!via `PlayFromStart`)
            (:`Update`
              (`SceneComponent.K2_SetRelativeRotation` (`self.Scene1`) (`KismetMathLibrary.MakeRotator` 0.0 0.0 (`KismetMathLibrary.Lerp` (`self.currentYaw`) (`KismetMathLibrary.SelectFloat` -90.0 90.0 (`self.isFront`)) _alpha)) false false))
            (:`Finished`
              (`self.SetCloseTimer`))))
        (:`then_1`
          (`GameplayStatics.PlaySound2D` "/Game/Sound/DoorKick.DoorKick" 1.0 1.0 0.0 null null))
        (:`then_2`
          (set `self.isOpen` true))))))

(event `StopOpen`
  (`|ExecutionSequence`
    (:`then_0`
      (`TimelineComponent.Stop` (`self.TL_KickOpen`))
      (`TimelineComponent.Stop` (`self.TL_NormalOpen`)))
    (:`then_1`
      (bind _opensound (`self.openSound`)
        (:`then`
          (`ActorComponent.K2_DestroyComponent` _opensound)
          (set `self.openSound` null))
        (:`else`)))))

(event `Close`
  (`|ExecutionSequence`
    (:`then_0`
      (bind (_direction _alpha) (`Timeline|TL_Close` :!via `PlayFromStart`)
        (:`Update`
          (`SceneComponent.K2_SetRelativeRotation` (`self.Scene1`) (`KismetMathLibrary.MakeRotator` 0.0 0.0 (`KismetMathLibrary.Lerp` (`KismetMathLibrary.SelectFloat` -90.0 90.0 (`self.isFront`)) 0.0 _alpha)) false false))
        (:`Finished`
          (set `self.isOpen` false))))
    (:`then_1`
      (`GameplayStatics.PlaySound2D` "/Game/Sound/DoorOpen.DoorOpen" 1.0 1.0 0.0 null null))))

(event `SetCloseTimer`
  (`KismetSystemLibrary.K2_SetTimerDelegate` (`|CreateDelegate` :!event `Close`) (`self.closeTime`)))

(fn `GetIsFront`
  (params (location :type "Vector Structure"))
  (returns (ReturnValue :type Boolean))
  (return (>= (`KismetMathLibrary.Dot_VectorVector` (`self.GetActorForwardVector`) (`KismetMathLibrary.GetForwardVector` (`KismetMathLibrary.FindLookAtRotation` (`self.K2_GetActorLocation`) location))) 0.0)))

(fn `UserConstructionScript`)